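; ExplosionRock is an actor that explodes and destroys itself when another actor begins overlapping it.
; The overlap spawns an enlarged P_Explosion particle at the Cuberock component's location, then destroys the actor.
; On destruction, it spawns Blueprint_Effect_Explosion there and calls Explosion.
; Explosion applies a zero-vector impulse to its own static mesh component, so it adds no push.
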(event EventBeginPlay)

(event Collision|EventActorBeginOverlap
  (params (OtherActor :type Actor%20Object%20Reference))
  (Effects|SpawnEmitteratLocation "/Game/StarterContent/Particles/P_Explosion.P_Explosion" (Transformation|GetWorldLocation (Variables|Default|GetCuberock)) "0, 0, 0" "10.000000,10.000000,10.000000")
  (Actor|DestroyActor))

(event EventTick
  (params (DeltaSeconds :type Float%20%28single-precision%29)))

(event EventDestroyed
  (Game|SpawnActorfromClass "/Game/StarterContent/Blueprints/Blueprint_Effect_Explosion.Blueprint_Effect_Explosion_C" (Math|Conversions|ToTransform(Vector) (Transformation|GetWorldLocation (Variables|Default|GetCuberock))) "Undefined" "MultiplyWithRoot" 0 0)
  (CallFunction|Explosion))

(fn ConstructionScript)

(fn Explosion
  (for _array_element (Utilities|Array|MakeArray (Actor|GetComponentbyClass "/Script/Engine.StaticMeshComponent"))
    (Physics|AddImpulse _array_element "0, 0, 0" "None" false)))