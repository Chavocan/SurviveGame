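; BPC_ItemsContainerMaster is a base item container component that stores items in an array of slots.
; AddItemOnServer calls FAddItem, which writes the item into the first slot whose ItemID is 0 and does nothing if none is free.
; After a successful write, FUpdateUI switches on container type and, for Inventory, sends the slot index and item info to the owner through UpdateItemMessage.
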(event Custom|AddItemOnServer
  (params (Item :type S%20Item%20Structure%20Structure))
  (CallFunction|FAddItem Item))

(fn FFindEmptySlot
  (bind (_array_element _array_index) (Utilities|Array|ForEachLoopwithBreak (Variables|Default|GetItems) :!label _label)
    (:LoopBody
      (if (== (.ItemID (Utilities|Struct|BreakS_ItemStructure _array_element)) 0)
        (LocalVariables|SetLocalEmptySlotIndex _array_index)
        (LocalVariables|SetFoundEmptySlot? true)
        (goto _label Break)))
    (:Completed
      (return (LocalVariables|GetFoundEmptySlot?) (LocalVariables|GetLocalEmptySlotIndex)))))

(fn FAddItem
  (params (Item :type S%20Item%20Structure%20Structure))
  (LocalVariables|SetLocalItemInfo Item)
  (bind (_success_ _emptyindex) (CallFunction|FFindEmptySlot))
  (if _success_
    (LocalVariables|SetLocalEmptyIndex _emptyindex)
    (Utilities|Array|SetArrayElem (Variables|Default|GetItems) (LocalVariables|GetLocalEmptyIndex) (LocalVariables|GetLocalItemInfo))
    (CallFunction|FUpdateUI (LocalVariables|GetLocalEmptyIndex) (LocalVariables|GetLocalItemInfo))))

(fn FUpdateUI
  (params (Index :type Integer) (ItemInfo :type S%20Item%20Structure%20Structure))
  (switch Utilities|FlowControl|Switch|SwitchonE_ContainerType (Variables|Default|GetContainerType)
    (:NewEnumerator0
      (Class|BPISurvivalCharacter|UpdateItem(Message) (Components|GetOwner) (Variables|Default|GetContainerType) Index ItemInfo))))